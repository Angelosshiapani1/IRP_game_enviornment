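; Interaction component that finds interactable actors in front of its owner and lets the player interact with or inspect them.
; A looping 0.2-second timer runs a forward sphere trace, keeping hits that implement BPI_Interaction as the target and showing their look-at message in an on-screen widget.
; Interact and Inspect Enhanced Input actions call the target's interface functions.
; The trace still draws debug shapes despite its CapsuleTrace name.
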(event Custom|BeginInteraction
  (Utilities|Time|SetTimerbyEvent (delegate Custom|UpdateInteraction) 0.2 true))

(event Custom|UpdateInteraction
  (CallFunction|CapsuleTrace))

(event Input|EnhancedActionEvents|EnhancedInputActionIA_Interact
  (params (ActionValue :type Boolean) (ElapsedSeconds :type Float%20%28double-precision%29) (TriggeredSeconds :type Float%20%28double-precision%29) (InputAction :type Input%20Action%20Object%20Reference :default "/Game/FirstPerson/Input/Actions/IA_Interact.IA_Interact"))
  (:Started
    (bind _targetactor (Variables|Default|GetTargetActor)
      (:then
        (Class|BPIInteraction|Interactwith(Message) _targetactor (CallFunction|GetMyPlayer))
        (Development|PrintString "Interacting"))
      (:else))))

(event Input|EnhancedActionEvents|EnhancedInputActionIA_Inspect
  (params (ActionValue :type Boolean) (ElapsedSeconds :type Float%20%28double-precision%29) (TriggeredSeconds :type Float%20%28double-precision%29) (InputAction :type Input%20Action%20Object%20Reference :default "/Game/FirstPerson/Input/Actions/IA_Inspect.IA_Inspect"))
  (:Started
    (bind _targetactor (Variables|Default|GetTargetActor)
      (:then
        (Class|BPIInteraction|Inspect(Message) _targetactor)
        (Development|PrintString "Inspecting" true true "(R=1.000000,G=0.000000,B=0.992671,A=1.000000)"))
      (:else))))

(event EventBeginPlay
  (CallFunction|CreateInteractMessage)
  (CallFunction|BeginInteraction))

(fn CreateInteractMessage
  (bind _returnvalue (UserInterface|CreateWidget "/Game/Interaction/UI/WB_InteractMessage.WB_InteractMessage_C"))
  (bind _output_get (Variables|Default|SetWB_InteractMessage _returnvalue))
  (UserInterface|Viewport|AddtoViewport _output_get 0))

(fn CapsuleTrace
  (bind _returnvalue (Components|GetOwner))
  (bind _returnvalue_2 (Transformation|GetActorLocation _returnvalue))
  (bind (_outhit _returnvalue_3) (Collision|SphereTraceByChannel _returnvalue_2 (+ _returnvalue_2 (* (Transformation|GetActorForwardVector _returnvalue) 1.5e+02)) 8e+01 "TraceTypeQuery3" false 0 "ForOneFrame"))
  (if _returnvalue_3
    (if (Utilities|DoesObjectImplementInterface (.HitActor (Collision|BreakHitResult _outhit)) "/Game/Interaction/BPI_Interaction.BPI_Interaction_C")
      (bind _output_get (Variables|Default|SetTargetActor (.HitActor (Collision|BreakHitResult _outhit))))
      (bind _message (Class|BPIInteraction|Lookat(Message) _output_get))
      (Default|SetMessage (Variables|Default|GetWB_InteractMessage) _message)
      (else
        (Variables|Default|SetTargetActor 0)
        (Default|SetMessage (Variables|Default|GetWB_InteractMessage))))
    (else
      (Variables|Default|SetTargetActor 0)
      (Default|SetMessage (Variables|Default|GetWB_InteractMessage)))))