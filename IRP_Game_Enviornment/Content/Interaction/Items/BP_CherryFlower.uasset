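; BP_CherryFlower is an inspectable item whose details come from the data table row referenced by its BPCItemData component.
; Inspect spawns a BP_Inspect_Base far out in the world and passes it the mesh, materials, name, description, weight and value.
; LookAt returns a "Look at" prompt with the item's name.
; The Interactwith event is empty.
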(event EventBeginPlay)

(event Collision|EventActorBeginOverlap
  (params (OtherActor :type Actor%20Object%20Reference)))

(event EventTick
  (params (DeltaSeconds :type Float%20%28single-precision%29)))

(event EventInspect
  (params (InspectInfo :type S%20Inspect%20Info%20Structure))
  (bind _bpc_itemdata (Variables|Default|GetBPC_ItemData))
  (bind _itemmesh (Variables|Default|GetItemMesh))
  (bind _itemdata (Variables|/Game/Interaction/ItemData/BPC_ItemData.BPC_ItemData_C|GetItemData _bpc_itemdata))
  (bind (_datatable _rowname) (Utilities|Struct|BreakDataTableRowHandle _itemdata))
  (bind _returnvalue (Utilities|GetDataTableRow _datatable _rowname)
    (:then
      (bind _returnvalue_2 (Game|SpawnActorfromClass "/Game/Interaction/Inspect/BP_Inspect_Base.BP_Inspect_Base_C" (Math|Transform|MakeTransform "1000000000.000000,0.000000,0.000000" "0, 0, 0" "1.000000,1.000000,1.000000") "Undefined" "MultiplyWithRoot" 0 0))
      (Default|Inspect _returnvalue_2 (Utilities|Struct|MakeS_InspectInfo (Variables|/Script/Engine.StaticMeshComponent|GetStaticMesh _itemmesh) (Rendering|Material|GetMaterials _itemmesh) (.ItemName (Utilities|Struct|BreakS_ItemInfo _returnvalue)) (.ItemDescription (Utilities|Struct|BreakS_ItemInfo _returnvalue)) (.ItemWeight (Utilities|Struct|BreakS_ItemInfo _returnvalue)) (Math|Conversions|ToInteger(Byte) (.ItemValue (Utilities|Struct|BreakS_ItemInfo _returnvalue))))))))

(event EventInteractwith
  (params (PlayerCharacture :type BP%20First%20Person%20Character%20Object%20Reference)))

(fn ConstructionScript)

(fn Lookat
  (bind _bpc_itemdata (Variables|Default|GetBPC_ItemData))
  (bind _itemdata (Variables|/Game/Interaction/ItemData/BPC_ItemData.BPC_ItemData_C|GetItemData _bpc_itemdata))
  (bind (_datatable _rowname) (Utilities|Struct|BreakDataTableRowHandle _itemdata))
  (bind _returnvalue (Utilities|GetDataTableRow _datatable _rowname)
    (:then
      (return (Utilities|Text|FormatText "Look at {Item}" (.ItemName (Utilities|Struct|BreakS_ItemInfo _returnvalue)))))))