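; Inspectable kusarigama prop that the player can bring into view and rotate with the mouse.
; Interact fires once, locks movement and look, shows the cursor and plays a Timeline lerping the mesh to the Kusarigama component transform on BP_FirstPersonCharacter.
; While inspecting, both mouse axes feed one local roll and pitch rotation.
; Q re-arms Interact, restores player control and reverses the Timeline to return the prop.
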(event EventBeginPlay
  (bind _kusarigama (Variables|Default|GetKusarigama))
  (bind _output_get (Variables|Default|SetOriginal%20location (Transformation|GetWorldLocation _kusarigama)))
  (Variables|Default|SetOriginal%20rotation (Transformation|GetWorldRotation _kusarigama))
  (Input|EnableInput (Game|GetPlayerController 0)))

(event EventInteract
  (Utilities|FlowControl|DoOnce false
    (:Completed
      (Variables|/Script/Engine.PlayerController|SetbShowMouseCursor (Game|GetPlayerController 0) true)
      (Variables|Default|SetKusarigama%20inspect? true)
      (bind _asbp_first_person_character (Utilities|Casting|CastToBP_FirstPersonCharacter (Game|GetPlayerCharacter 0)))
      (Pawn|Components|CharacterMovement|DisableMovement (Variables|/Script/Engine.Character|GetCharacterMovement (Game|GetPlayerCharacter 0)))
      (Input|SetIgnoreLookInput (Game|GetPlayerController 0) true)
      (bind _newtrack_0 (Timeline|Timeline Play)
        (:Update
          (Transformation|SetWorldTransform (Variables|Default|GetKusarigama) (Math|Transform|MakeTransform (Math|Vector|Lerp(Vector) (stale EventBeginPlay _output_get) (.location (Transformation|GetWorldTransform (Variables|/Game/FirstPerson/Blueprints/BP_FirstPersonCharacter.BP_FirstPersonCharacter_C|GetKusarigama _asbp_first_person_character))) _newtrack_0) (Math|Rotator|Lerp(Rotator) (Variables|Default|GetOriginal%20rotation) (.rotation (Transformation|GetWorldTransform (Variables|/Game/FirstPerson/Blueprints/BP_FirstPersonCharacter.BP_FirstPersonCharacter_C|GetKusarigama _asbp_first_person_character))) _newtrack_0) "1.000000,1.000000,1.000000") false false))))))

(event Input|MouseEvents|MouseX
  (params (AxisValue :type Float%20%28single-precision%29))
  (if (Variables|Default|GetKusarigama%20inspect?)
    (Transformation|AddLocalRotation (Variables|Default|GetKusarigama) (Math|Rotator|MakeRotator (* AxisValue 0.4) (* (stale Input|MouseEvents|MouseY AxisValue) -0.4) 0.0) false false)))

(event Input|MouseEvents|MouseY
  (params (AxisValue :type Float%20%28single-precision%29))
  (if (Variables|Default|GetKusarigama%20inspect?)
    (Transformation|AddLocalRotation (Variables|Default|GetKusarigama) (Math|Rotator|MakeRotator (* (stale Input|MouseEvents|MouseX AxisValue) 0.4) (* AxisValue -0.4) 0.0) false false)))

(event Input|KeyboardEvents|Q
  (params (Key :type Key%20Structure :default "None"))
  (bind _returnvalue (Game|GetPlayerController 0))
  (:Pressed
    (Utilities|FlowControl|Sequence
      (:then_0
        (Utilities|FlowControl|DoOnce false) ; enters at Reset
      )
      (:then_1
        (Variables|Default|SetKusarigama%20inspect? false)
        (Pawn|Components|CharacterMovement|SetMovementMode (Variables|/Script/Engine.Character|GetCharacterMovement (Game|GetPlayerCharacter 0)) "MOVE_Walking" 0)
        (Variables|/Script/Engine.PlayerController|SetbShowMouseCursor _returnvalue false)
        (Input|ResetIgnoreLookInput _returnvalue)
        (Input|SetInputModeGameOnly _returnvalue false)
        (bind _newtrack_0 (Timeline|Timeline Reverse)
          (:Update
            (Transformation|SetWorldTransform (Variables|Default|GetKusarigama) (Math|Transform|MakeTransform (Math|Vector|Lerp(Vector) (stale EventBeginPlay _output_get) (.location (Transformation|GetWorldTransform (Variables|/Game/FirstPerson/Blueprints/BP_FirstPersonCharacter.BP_FirstPersonCharacter_C|GetKusarigama (stale EventInteract _asbp_first_person_character)))) _newtrack_0) (Math|Rotator|Lerp(Rotator) (Variables|Default|GetOriginal%20rotation) (.rotation (Transformation|GetWorldTransform (Variables|/Game/FirstPerson/Blueprints/BP_FirstPersonCharacter.BP_FirstPersonCharacter_C|GetKusarigama (stale EventInteract _asbp_first_person_character)))) _newtrack_0) "1.000000,1.000000,1.000000") false false)))))))

(fn ConstructionScript)