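; BP_NoteMaker is an overlap-triggered actor that lets the player view a note card on screen.
; Entering its overlap enables input and writes the actor's NoteCard to the first-person character's NoteIndex.
; While input is enabled, the E key flip-flops between creating and removing a NoteCardDisplay widget.
; Leaving the overlap disables input and removes the widget.
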(event Collision|EventActorBeginOverlap
  (params (OtherActor :type Actor%20Object%20Reference))
  (Input|EnableInput (Game|GetPlayerController 0))
  (bind _asbp_first_person_character (Utilities|Casting|CastToBP_FirstPersonCharacter (Game|GetPlayerCharacter 0)))
  (Variables|/Game/FirstPerson/Blueprints/BP_FirstPersonCharacter.BP_FirstPersonCharacter_C|SetNoteIndex _asbp_first_person_character (Variables|Default|GetNoteCard)))

(event Collision|EventActorEndOverlap
  (params (OtherActor :type Actor%20Object%20Reference))
  (Input|DisableInput 0)
  (Widget|RemovefromParent (stale Input|KeyboardEvents|E _returnvalue)))

(event Input|KeyboardEvents|E
  (params (Key :type Key%20Structure))
  (:Pressed
    (Utilities|FlowControl|FlipFlop
      (:A
        (bind _returnvalue (UserInterface|CreateWidget "/Game/UI_Blueprints/Note_BP/NoteCardDisplay.NoteCardDisplay_C"))
        (UserInterface|Viewport|AddtoViewport _returnvalue 0))
      (:B
        (Widget|RemovefromParent _returnvalue)))))

(fn ConstructionScript)